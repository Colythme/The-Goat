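; Lens flare source actor that drives a set of screen-space flare element widgets.
; On BeginPlay it creates one widget per FlareElements struct, gives it a dynamic material (custom, or base additive/translucent) and passes in that element's settings.
; Each tick it zeroes widget occlusion beyond max distance or when a Visibility trace to the camera is blocked, otherwise applies per-element distance cutoffs.
; Moveable flares also update widget source location.
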(event `self.ReceiveTick`
  (params (DeltaSeconds :type "Float (single-precision)"))
  ;[1 1 1] Every Frame Perform the occlusion test
  (`self.UpdateFlareVisibility`)
  (if (`self.Flare Moveable?`)
    (for _array_element (`self.Flare Elements`)
      (set `/Game/LensFlareTool/Blueprints/FlareWidget.ParentLocation` (`self.K2_GetActorLocation`) (`.FlareWidget_38_76CA7C9641CC97FC2D7B4489673481E6` (break `/Game/LensFlareTool/Blueprints/Struct_FlareItem` _array_element))))))

(event `self.ReceiveBeginPlay`
  ;[1 1 1] At the start initialize the struct array contents
  (`self.InitiateFlares`))

(fn `InitiateFlares`
  ;[1 1 1] For Each Flare Element
  (for (_array_element _array_index) (`self.Flare Elements`)
    ;[1 1 1] Create new flare element widget
    (bind _returnvalue (`|CreateWidget` "/Game/LensFlareTool/Blueprints/FlareWidget.FlareWidget_C" (`GameplayStatics.GetPlayerController` 0)))
    (bind (_color _flarewidget _flarelocation _ismaterialadditive _fadoutedgedistance _elementmaximumdistance _fadeout_enableshrinking _fadeout_enableopacityfade _fadeout_flarelocation _material _screenpositionoffset _globalsizemultiplier _initialspriteangle _activerotationamount _enableorbitrotation _enableslocationscaling _locationscalinginfluence _locationscalingcentersize _locationscalingedgesize _enablelocationbasedopacity _locopacitycenteropacity _locopacityedgeopacity _locopacityinfluence) (break `/Game/LensFlareTool/Blueprints/Struct_FlareItem` _array_element))
    (bind _struct_flareitem (make `/Game/LensFlareTool/Blueprints/Struct_FlareItem` _color _returnvalue _flarelocation _ismaterialadditive _fadoutedgedistance _elementmaximumdistance _fadeout_enableshrinking _fadeout_enableopacityfade _fadeout_flarelocation _material _screenpositionoffset _globalsizemultiplier _initialspriteangle _activerotationamount _enableorbitrotation _enableslocationscaling _locationscalinginfluence _locationscalingcentersize _locationscalingedgesize _enablelocationbasedopacity _locopacitycenteropacity _locopacityedgeopacity _locopacityinfluence))
    ;[1 1 1] Add that widget to the flare element struct
    (`KismetArrayLibrary.Array_Set` (`self.Flare Elements`) _array_index _struct_flareitem)
    (bind (_color_2 _flarewidget_2 _flarelocation_2 _ismaterialadditive_2 _fadoutedgedistance_2 _elementmaximumdistance_2 _fadeout_enableshrinking_2 _fadeout_enableopacityfade_2 _fadeout_flarelocation_2 _material_2 _screenpositionoffset_2 _globalsizemultiplier_2 _initialspriteangle_2 _activerotationamount_2 _enableorbitrotation_2 _enableslocationscaling_2 _locationscalinginfluence_2 _locationscalingcentersize_2 _locationscalingedgesize_2 _enablelocationbasedopacity_2 _locopacitycenteropacity_2 _locopacityedgeopacity_2 _locopacityinfluence_2) (break `/Game/LensFlareTool/Blueprints/Struct_FlareItem` _struct_flareitem))
    ;[1 1 1] Initialize each widget. This means passing most of the element struct information, and adding the material, setting the color and a few other things
    (if (`KismetSystemLibrary.IsValid` _material_2)
      (bind _returnvalue_2 (`KismetMaterialLibrary.CreateDynamicMaterialInstance` _material_2))
      (set `/Game/LensFlareTool/Blueprints/FlareWidget.CurrentMaterial` _returnvalue_2 _flarewidget_2)
      (elif _ismaterialadditive_2
        (bind _returnvalue_3 (`KismetMaterialLibrary.CreateDynamicMaterialInstance` "/Game/LensFlareTool/Materials/M_BaseFlareMaterial_Additive.M_BaseFlareMaterial_Additive"))
        (set `/Game/LensFlareTool/Blueprints/FlareWidget.CurrentMaterial` _returnvalue_3 _flarewidget_2)
        (else
          (bind _returnvalue_4 (`KismetMaterialLibrary.CreateDynamicMaterialInstance` "/Game/LensFlareTool/Materials/M_BaseFlareMaterial_Trans.M_BaseFlareMaterial_Trans"))
          (set `/Game/LensFlareTool/Blueprints/FlareWidget.CurrentMaterial` _returnvalue_4 _flarewidget_2))))
    (bind (_x _y) (`KismetMathLibrary.BreakVector2D` _fadoutedgedistance_2))
    (`/Game/LensFlareTool/Blueprints/FlareWidget.Initialize` _flarewidget_2 _flarelocation_2 (`SceneComponent.K2_GetComponentLocation` (`self.DefaultSceneRoot`)) _x _y _elementmaximumdistance_2 _locationscalingcentersize_2 _locationscalingedgesize_2 _locationscalinginfluence_2 _enableslocationscaling_2 _screenpositionoffset_2 _enableorbitrotation_2 _initialspriteangle_2 _globalsizemultiplier_2 _fadeout_enableshrinking_2 _fadeout_enableopacityfade_2 _fadeout_flarelocation_2 _enablelocationbasedopacity_2 _locopacitycenteropacity_2 _locopacityedgeopacity_2 _locopacityinfluence_2 _activerotationamount_2 (`.SpecifiedColor` (break `SlateColor` _color_2)) _ismaterialadditive_2)
    (`KismetArrayLibrary.Array_Add` (`self.WidgetList`) _flarewidget_2)
    (set `/Game/LensFlareTool/Blueprints/FlareWidget.Occlusion Update Speed` (`self.Occlusion Update Speed`) _flarewidget_2)))

(fn `UpdateFlareVisibility`
  (bind _widgetlist (`self.WidgetList`))
  (bind _playercameramanager (`PlayerController.PlayerCameraManager` (`GameplayStatics.GetPlayerController` 0)))
  (bind _returnvalue (`self.GetDistanceTo` _playercameramanager))
  ;[1 1 1] First check the source BP distance to the camera.  If it's past max, kill the check completely
  (if (> _returnvalue (`self.Global Maximum Distance`))
    ;[1 1 1] If it's beyond max range clear the occlusion controlling variable in each flare element
    (for _array_element _widgetlist :!label _label
      (set `/Game/LensFlareTool/Blueprints/FlareWidget.OcclusionMult` 0.0 _array_element))
    (else
      ;[1 1 1] Establish if the source is then visible
      (bind (_outhit _returnvalue_2) (`KismetSystemLibrary.LineTraceSingle` (`SceneComponent.K2_GetComponentLocation` (`self.DefaultSceneRoot`)) (`SceneComponent.K2_GetComponentLocation` (`PlayerCameraManager.TransformComponent` _playercameramanager)) "TraceTypeQuery1"))
      ;[1 1 1] Then if not visible occlude
      (if _returnvalue_2
        (goto _label)
        (else
          ;[1 1 1] Then per element, check the fade distance, and adjust accordingly
          (for _array_element_2 _widgetlist
            (if (> _returnvalue (`/Game/LensFlareTool/Blueprints/FlareWidget.FadeDistance` _array_element_2))
              (set `/Game/LensFlareTool/Blueprints/FlareWidget.OcclusionMult` 0.0 _array_element_2)
              (else
                (set `/Game/LensFlareTool/Blueprints/FlareWidget.OcclusionMult` 1.0 _array_element_2)))))))))

(fn `UserConstructionScript`)