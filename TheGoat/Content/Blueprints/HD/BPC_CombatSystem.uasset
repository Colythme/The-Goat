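; Player combat component for BP_Player, handling light and heavy melee combos, dodge, block and enemy target lock.
; Attack input drives indexed montage chains with a short re-press buffer, saved light follow-ups and hold-to-charge heavies, spending stamina from data-table rows.
; A camera sphere trace picks the lock target, steering rotation and switching dodge from montage to timer-driven velocity.
; The timer-looped sword sphere trace only draws debug, without processing hits.
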(event `EnhancedInput|/Game/Input/Actions/IA_HLock`
  (params (ActionValue :type Boolean) (ElapsedSeconds :type "Float (double-precision)") (TriggeredSeconds :type "Float (double-precision)") (InputAction :type "InputAction Object Reference" :default "/Game/Input/Actions/IA_HLock.IA_HLock"))
  (bind _returnvalue (`Actor.GetTransform` (`self.Target Lock Actor`)))
  (bind _transformcomponent (`PlayerCameraManager.TransformComponent` (`GameplayStatics.GetPlayerCameraManager` 0)))
  (bind _charactermovement (`Character.CharacterMovement` (`self.Player BP`)))
  (bind _charactermovement_2 (`Character.CharacterMovement` (`self.Player BP`)))
  (bind (_returnvalue_x _returnvalue_y _returnvalue_z) (`KismetMathLibrary.BreakVector` (`SceneComponent.K2_GetComponentLocation` _transformcomponent)))
  (bind _returnvalue_2 (`KismetMathLibrary.MakeVector` _returnvalue_x _returnvalue_y (+ _returnvalue_z 20.0)))
  (:`Started`
    (`self.Target Lock Actor`
      (:`then`
        (set `self.Is Player Locking?` false)
        (set `self.Target Lock Actor` null)
        (set `CharacterMovementComponent.bOrientRotationToMovement` true _charactermovement)
        (set `CharacterMovementComponent.bUseControllerDesiredRotation` false _charactermovement)
        (`Actor.K2_DestroyActor` (`self.Target Lock Widget`)))
      (:`else`
        (bind (_outhit _returnvalue_3) (`KismetSystemLibrary.SphereTraceSingleForObjects` :`Start` _returnvalue_2 :`End` (+ _returnvalue_2 (* (`KismetMathLibrary.GetForwardVector` (`SceneComponent.K2_GetComponentRotation` _transformcomponent)) 1500.0)) :`Radius` 150.0 :`ObjectTypes` (`|MakeArray` "ObjectTypeQuery3" :!type "EObjectTypeQuery Enum") :`DrawDebugType` "ForDuration" :`DrawTime` 2.0))
        (if _returnvalue_3
          (set `self.Is Player Locking?` true)
          (bind (_bblockinghit _binitialoverlap _time _distance _location _impactpoint _normal _impactnormal _physmat _hitactor) (`GameplayStatics.BreakHitResult` _outhit))
          (if (`Actor.ActorHasTag` _hitactor "Enemy")
            (set `self.Target Lock Actor` _hitactor)
            (set `CharacterMovementComponent.bOrientRotationToMovement` false _charactermovement_2)
            (set `CharacterMovementComponent.bUseControllerDesiredRotation` true _charactermovement_2)
            (bind _returnvalue_4 (`|SpawnActorFromClass` "/Game/Blueprints/HD/AC_TargetLockWidget.AC_TargetLockWidget_C" (`KismetMathLibrary.MakeTransform` (`KismetMathLibrary.MakeVector` (.x (.location _returnvalue)) (.y (.location _returnvalue)) (+ (.z (.location _returnvalue)) 20.0)) (.rotation _returnvalue)) "Undefined" "MultiplyWithRoot" null null))
            (bind _output_get (set `self.Target Lock Widget` _returnvalue_4))
            (`Actor.K2_AttachToActor` _output_get (`self.Target Lock Actor`) "None" "SnapToTarget" "SnapToTarget" "SnapToTarget" true)))))))

(event `EnhancedInput|/Game/Input/Actions/IA_HLightAttack`
  (params (ActionValue :type Boolean) (ElapsedSeconds :type "Float (double-precision)") (TriggeredSeconds :type "Float (double-precision)") (InputAction :type "InputAction Object Reference" :default "/Game/Input/Actions/IA_HLightAttack.IA_HLightAttack"))
  (:`Triggered`
    (set `self.Current Press Attack Is Light?` true)
    (if (`self.Can Attack?`) :!label _label
      (if (`/Game/Blueprints/HD/BP_Player.Have Stamina?` (`self.Player BP`))
        (if (not (`self.In Attack Buffer?`))
          (set `self.Is Current Attack Light?` (`self.Current Press Attack Is Light?`))
          (set `/Game/Blueprints/HD/BP_Player.Can Move?` false (`self.Player BP`))
          (`self.Force Stop Dodging ABP`)
          (`self.Attack Combo Input`))))))

(event `Attack Combo Input`
  (if (`self.Is Attacking?`)
    (if (`self.Can Play Next Attack Anim?`)
      (set `self.Save Attack?` false)
      (set `self.Can Play Next Attack Anim?` false :!label _label_2)
      (`|ExecutionSequence`
        (:`then_0`
          (set `self.In Attack Buffer?` true)
          (`KismetSystemLibrary.Delay` 0.4)
          (set `self.In Attack Buffer?` false))
        (:`then_1`
          (if (`self.Is Current Attack Light?`)
            (`self.Deal Light Attack`)
            (else
              (`self.Deal Heavy Attack Charge`)))))
      (elif (`self.Is Current Attack Light?`)
        (set `self.Save Attack?` true)
        (else
          (set `self.Save Attack?` false))))
    (else
      (set `self.Is Attacking?` true)
      (goto _label_2))))

(event `Attack Combo Auto`
  (if (`self.Save Attack?`)
    (set `self.Save Attack?` false)
    (goto _label_2)))

(event `Stop Combo`
  (set `self.Is Attacking?` false)
  (set `self.Save Attack?` false)
  (set `self.Can Rotate?` false)
  (set `self.Can Play Next Attack Anim?` false)
  (set `self.Light Attack Index` 0)
  (set `self.Heavy Attack Index` 0))

(event `Light Attack Combo 01`
  (`/Engine/EditorBlueprintResources/StandardMacros.DoOnce` false :!label _label_3
    (:`Completed`
      (`KismetSystemLibrary.Delay` 0.1)
      (`|PlayMontage` (`self.Player Mesh`) "/Game/Animations/Samurai/Raw_UE4/Attack/LightAttack/LightAttackCombo_01_Montage.LightAttackCombo_01_Montage"
        (:`then`
          (set `self.Light Attack Index` 1)
          (goto _label_3 :!via `Reset`))))))

(event `Light Attack Combo 02`
  (`/Engine/EditorBlueprintResources/StandardMacros.DoOnce` false :!label _label_4
    (:`Completed`
      (`KismetSystemLibrary.Delay` 0.1)
      (`|PlayMontage` (`self.Player Mesh`) "/Game/Animations/Samurai/Raw_UE4/Attack/LightAttack/LightAttackCombo_02_Montage.LightAttackCombo_02_Montage"
        (:`then`
          (set `self.Light Attack Index` 2)
          (goto _label_4 :!via `Reset`))))))

(event `Light Attack Combo 03`
  (`/Engine/EditorBlueprintResources/StandardMacros.DoOnce` false :!label _label_5
    (:`Completed`
      (`KismetSystemLibrary.Delay` 0.1)
      (`|PlayMontage` (`self.Player Mesh`) "/Game/Animations/Samurai/Raw_UE4/Attack/LightAttack/LightAttackCombo_03_Montage.LightAttackCombo_03_Montage"
        (:`then`
          (set `self.Light Attack Index` 3)
          (goto _label_5 :!via `Reset`))))))

(event `Light Attack Combo 04`
  (`/Engine/EditorBlueprintResources/StandardMacros.DoOnce` false :!label _label_6
    (:`Completed`
      (`KismetSystemLibrary.Delay` 0.1)
      (`|PlayMontage` (`self.Player Mesh`) "/Game/Animations/Samurai/Raw_UE4/Attack/LightAttack/LightAttackCombo_04_Montage.LightAttackCombo_04_Montage"
        (:`then`
          (set `self.Light Attack Index` 4)
          (goto _label_6 :!via `Reset`))))))

(event `Light Attack Combo 05`
  (`/Engine/EditorBlueprintResources/StandardMacros.DoOnce` false :!label _label_7
    (:`Completed`
      (`KismetSystemLibrary.Delay` 0.1)
      (`|PlayMontage` (`self.Player Mesh`) "/Game/Animations/Samurai/Raw_UE4/Attack/LightAttack/LightAttackCombo_05_Montage.LightAttackCombo_05_Montage"
        (:`then`
          (set `self.Light Attack Index` 5)
          (goto _label_7 :!via `Reset`))))))

(event `Heavy Attack Combo 01 Charge`
  (`KismetSystemLibrary.Delay` 0.1)
  (`|PlayMontage` (`self.Player Mesh`) "/Game/Animations/Samurai/Raw_UE4/Attack/HeavyAttack/HeavyAttackCombo_01_Charge_Montage.HeavyAttackCombo_01_Charge_Montage"))

(event `Heavy Attack Combo 01 Release`
  (`/Engine/EditorBlueprintResources/StandardMacros.DoOnce` false :!label _label_8
    (:`Completed`
      (`KismetSystemLibrary.Delay` 0.1)
      (`|PlayMontage` (`self.Player Mesh`) "/Game/Animations/Samurai/Raw_UE4/Attack/HeavyAttack/HeavyAttackCombo_01_Release_Montage.HeavyAttackCombo_01_Release_Montage"
        (:`then`
          (set `self.Heavy Attack Index` 1)
          (goto _label_8 :!via `Reset`))))))

(event `Heavy Attack Combo 02 Charge`
  (`KismetSystemLibrary.Delay` 0.1)
  (`|PlayMontage` (`self.Player Mesh`) "/Game/Animations/Samurai/Raw_UE4/Attack/HeavyAttack/HeavyAttackCombo_02_Charge_Montage.HeavyAttackCombo_02_Charge_Montage"))

(event `Heavy Attack Combo 02 Release`
  (`/Engine/EditorBlueprintResources/StandardMacros.DoOnce` false :!label _label_9
    (:`Completed`
      (`KismetSystemLibrary.Delay` 0.1)
      (`|PlayMontage` (`self.Player Mesh`) "/Game/Animations/Samurai/Raw_UE4/Attack/HeavyAttack/HeavyAttackCombo_02_Release_Montage.HeavyAttackCombo_02_Release_Montage"
        (:`then`
          (set `self.Heavy Attack Index` 2)
          (goto _label_9 :!via `Reset`))))))

(event `EnhancedInput|/Game/Input/Actions/IA_HHeavyAttack`
  (params (ActionValue :type Boolean) (ElapsedSeconds :type "Float (double-precision)") (TriggeredSeconds :type "Float (double-precision)") (InputAction :type "InputAction Object Reference" :default "/Game/Input/Actions/IA_HHeavyAttack.IA_HHeavyAttack"))
  (:`Triggered`
    (set `self.Current Press Attack Is Light?` false)
    (goto _label))
  (:`Completed`
    (if (`self.Is Attack Charging`)
      (`self.Deal Heavy Attack Release`))))

(event `Deal Light Attack`
  (switch `int` (`self.Light Attack Index`)
    (:`0`
      (`self.Light Attack Combo 01`)
      (`KismetSystemLibrary.Delay` 0.2)
      (`self.Attack Numeric Handler` "LightAttackCombo01"))
    (:`1`
      (`self.Light Attack Combo 02`)
      (`KismetSystemLibrary.Delay` 0.2)
      (`self.Attack Numeric Handler` "LightAttackCombo02"))
    (:`2`
      (`self.Light Attack Combo 03`)
      (`KismetSystemLibrary.Delay` 0.2)
      (`self.Attack Numeric Handler` "LightAttackCombo03"))
    (:`3`
      (`self.Light Attack Combo 04`)
      (`KismetSystemLibrary.Delay` 0.2)
      (`self.Attack Numeric Handler` "LightAttackCombo04"))
    (:`4`
      (`self.Light Attack Combo 05`)
      (`KismetSystemLibrary.Delay` 0.2)
      (`self.Attack Numeric Handler` "LightAttackCombo05"))))

(event `Deal Heavy Attack Charge`
  (set `self.Is Attack Charging` true)
  (switch `int` (`self.Heavy Attack Index`)
    (:`0`
      (`self.Heavy Attack Combo 01 Charge`))
    (:`1`
      (`self.Heavy Attack Combo 02 Charge`))))

(event `Deal Heavy Attack Release`
  (set `self.Is Attack Charging` false)
  (switch `int` (`self.Heavy Attack Index`)
    (:`0`
      (`self.Heavy Attack Combo 01 Release`)
      (`KismetSystemLibrary.Delay` 0.2)
      (`self.Attack Numeric Handler` "HeavyAttackCombo01"))
    (:`1`
      (`self.Heavy Attack Combo 02 Release`)
      (`KismetSystemLibrary.Delay` 0.2)
      (`self.Attack Numeric Handler` "HeavyAttackCombo02"))))

(event `Start Sword Trace`
  (bind _returnvalue (`KismetSystemLibrary.K2_SetTimerDelegate` (delegate `Sword Trace Loop`) 0.005 true))
  (set `self.Sword Trace Loop Timer` _returnvalue))

(event `Sword Trace Loop`
  (`KismetSystemLibrary.SphereTraceSingle` :`Start` (`SceneComponent.K2_GetComponentLocation` (`/Game/Blueprints/HD/BP_Player.Notachi Top Point` (`self.Player BP`))) :`End` (`SceneComponent.K2_GetComponentLocation` (`/Game/Blueprints/HD/BP_Player.Notachi Bottom Point` (`self.Player BP`))) :`Radius` 12.0 :`TraceChannel` "TraceTypeQuery1" :`DrawDebugType` "ForDuration" :`DrawTime` 0.5))

(event `Stop Sword Trace`
  (`KismetSystemLibrary.K2_ClearAndInvalidateTimerHandle` (`self.Sword Trace Loop Timer`)))

(event `EnhancedInput|/Game/Input/Actions/IA_HDodge`
  (params (ActionValue :type Boolean) (ElapsedSeconds :type "Float (double-precision)") (TriggeredSeconds :type "Float (double-precision)") (InputAction :type "InputAction Object Reference" :default "/Game/Input/Actions/IA_HDodge.IA_HDodge"))
  (:`Triggered`
    (if (`self.Can Dodge?`)
      (if (`/Game/Blueprints/HD/BP_Player.Have Stamina?` (`self.Player BP`))
        (`self.Force Stop Dodging ABP`)
        (`|ExecutionSequence`
          (:`then_0`
            (set `/Game/Blueprints/HD/BP_Player.Can Move?` true (`self.Player BP`))
            (`KismetSystemLibrary.Delay` 0.2)
            (`/Game/Blueprints/HD/BPC_PlayerStats.Decrease Current Stamina` (`self.BPC Player Stats`) 15.0))
          (:`then_1`
            (if (`self.Is Player Locking?`)
              (`/Game/Characters/Player/ABP_Player_Shin.StartDodgingABP` (`self.ABP Player`))
              (bind _direction_vector (`self.Get Input Direction Vector`))
              (bind _returnvalue (`KismetSystemLibrary.K2_SetTimerDelegate` (delegate `Move Foward`) (`GameplayStatics.GetWorldDeltaSeconds`) true))
              (set `self.Dodge Timer` _returnvalue)
              (else
                (`self.Rotate Actor to Last Input Direction`)
                (`Character.PlayAnimMontage` (`self.Player BP`) "/Game/Animations/Samurai/Raw_UE5/Dodge/Dodge_F.Dodge_F" 1.0 "None")))))))))

(event `Move Foward`
  (set `MovementComponent.Velocity` (* (stale `EnhancedInput|/Game/Input/Actions/IA_HDodge` _direction_vector) 700.0) (`self.Character Movement`)))

(event `Force Stop Dodging ABP`
  (set `/Game/Characters/Player/ABP_Player_Shin.Is Dodging?` false (`self.ABP Player`))
  (`self.Stop Dodge Movement`))

(event `Stop Dodge Movement`
  (`KismetSystemLibrary.K2_ClearAndInvalidateTimerHandle` (`self.Dodge Timer`)))

(event `EnhancedInput|/Game/Input/Actions/IA_HBlock`
  (params (ActionValue :type Boolean) (ElapsedSeconds :type "Float (double-precision)") (TriggeredSeconds :type "Float (double-precision)") (InputAction :type "InputAction Object Reference" :default "/Game/Input/Actions/IA_HBlock.IA_HBlock"))
  (:`Started`
    (if (`self.Can Defend?`)
      (if (`/Game/Blueprints/HD/BP_Player.Have Stamina?` (`self.Player BP`))
        (if (not (`self.Is Defending?`))
          (set `self.Is Defending?` true)
          (`/Game/Blueprints/HD/BP_Player.Stop Montage and Clean Paras` (`self.Player BP`))
          (set `CharacterMovementComponent.MaxWalkSpeed` 150.0 (`self.Character Movement`))
          (`self.Start Defending ABP`)))))
  (:`Completed`
    (set `self.Is Defending?` false)
    (`self.Stop Defending ABP`)
    (set `CharacterMovementComponent.MaxWalkSpeed` 300.0 (`self.Character Movement`))))

(event `Start Defending ABP`
  (set `/Game/Characters/Player/ABP_Player_Shin.Is Defending?` true (`self.ABP Player`)))

(event `Stop Defending ABP`
  (set `/Game/Characters/Player/ABP_Player_Shin.Is Defending?` false (`self.ABP Player`)))

(event `self.ReceiveBeginPlay`
  (bind _asbp_player (cast `/Game/Blueprints/HD/BP_Player` (`self.GetOwner`)))
  (bind _output_get (set `self.Player BP` _asbp_player))
  (set `self.Player Mesh` (`Character.Mesh` _output_get))
  (set `self.Character Movement` (`Character.CharacterMovement` _output_get))
  (bind _asabp_player_shin (cast `/Game/Characters/Player/ABP_Player_Shin` (`SkeletalMeshComponent.GetAnimInstance` (`self.Player Mesh`))))
  (set `self.ABP Player` _asabp_player_shin)
  (set `self.BPC Player Stats` (`/Game/Blueprints/HD/BP_Player.BPC_PlayerStats` (`self.Player BP`))))

(event `self.ReceiveTick`
  (params (DeltaSeconds :type "Float (single-precision)"))
  (bind (_last_rotation_vector_x _last_rotation_vector_y) (`KismetMathLibrary.BreakVector2D` (`/Game/Blueprints/HD/BP_Player.Last Rotation Vector` (`self.Player BP`))))
  (bind (_returnvalue_roll _returnvalue_pitch _returnvalue_yaw) (`KismetMathLibrary.BreakRotator` (`KismetMathLibrary.FindLookAtRotation` (`Actor.K2_GetActorLocation` (`self.Player BP`)) (`Actor.K2_GetActorLocation` (`self.Target Lock Actor`)))))
  (bind (_returnvalue_roll_2 _returnvalue_pitch_2 _returnvalue_yaw_2) (`KismetMathLibrary.BreakRotator` (`KismetMathLibrary.MakeRotFromX` (`KismetMathLibrary.GreaterGreater_VectorRotator` (`SceneComponent.GetForwardVector` (`/Game/Blueprints/HD/BP_Player.FollowCamera` (`self.Player BP`))) (`KismetMathLibrary.MakeRotFromX` (`KismetMathLibrary.MakeVector` _last_rotation_vector_y _last_rotation_vector_x))))))
  (`self.Target Lock Actor`
    (:`then`
      (`Controller.SetControlRotation` (`Pawn.GetController` (`self.Player BP`)) (`KismetMathLibrary.MakeRotator` _returnvalue_roll (+ _returnvalue_pitch -20.0) _returnvalue_yaw))
      ;[1 1 1] Cannot Keep Rotating to Locked Target When Sprinting
      (if (or (`self.Is Attacking?`) (not (`/Game/Blueprints/HD/BP_Player.Is Sprinting?` (`self.Player BP`))))
        (`self.Rotate to Locked Enemy`)))
    (:`else`
      (if (`self.Is Attacking?`)
        (if (`self.Can Rotate?`)
          (`Actor.K2_SetActorRotation` (`self.Player BP`) (`KismetMathLibrary.RInterpTo` (`Actor.K2_GetActorRotation` (`self.Player BP`)) (`KismetMathLibrary.MakeRotator` 0.0 0.0 _returnvalue_yaw_2) (`GameplayStatics.GetWorldDeltaSeconds`) 20.0) false))))))

(fn `Attack Numeric Handler`
  (params (`Attack Row Name` :type Name))
  (bind _returnvalue (`|GetDataTableRow` "/Game/Data/Data/PlayerAttack.PlayerAttack" `Attack Row Name`)
    (:`then`
      (`|ExecutionSequence`
        (:`then_0`
          (`/Game/Blueprints/HD/BPC_PlayerStats.Decrease Current Stamina` (`self.BPC Player Stats`) (`.StaminaCost_14_0D026A3849724EA2F0FB0DA87890E84E` (break `/Game/Data/S_PlayerAttack` _returnvalue))))))))

(fn `Get Input Direction Vector`
  (returns (`Direction Vector` :type "Vector Structure"))
  (bind (_last_rotation_vector_x _last_rotation_vector_y) (`KismetMathLibrary.BreakVector2D` (`/Game/Blueprints/HD/BP_Player.Last Rotation Vector` (`self.Player BP`))))
  (return (`KismetMathLibrary.GreaterGreater_VectorRotator` (`SceneComponent.GetForwardVector` (`/Game/Blueprints/HD/BP_Player.FollowCamera` (`self.Player BP`))) (`KismetMathLibrary.MakeRotFromX` (`KismetMathLibrary.MakeVector` _last_rotation_vector_y _last_rotation_vector_x)))))

(fn `Rotate Actor to Last Input Direction`
  (bind _direction_vector (`self.Get Input Direction Vector`))
  (bind (_returnvalue_roll _returnvalue_pitch _returnvalue_yaw) (`KismetMathLibrary.BreakRotator` (`KismetMathLibrary.MakeRotFromX` _direction_vector)))
  (`Actor.K2_SetActorRotation` (`self.Player BP`) (`KismetMathLibrary.MakeRotator` 0.0 0.0 _returnvalue_yaw) false))

(fn `Rotate to Locked Enemy`
  (bind _player_bp (`self.Player BP`))
  (bind (_returnvalue_roll _returnvalue_pitch _returnvalue_yaw) (`KismetMathLibrary.BreakRotator` (`KismetMathLibrary.FindLookAtRotation` (`Actor.K2_GetActorLocation` _player_bp) (`Actor.K2_GetActorLocation` (`self.Target Lock Actor`)))))
  (if (`self.Is Player Locking?`)
    (`Actor.K2_SetActorRotation` _player_bp (`KismetMathLibrary.RInterpTo` (`Actor.K2_GetActorRotation` (`self.Player BP`)) (`KismetMathLibrary.MakeRotator` 0.0 0.0 _returnvalue_yaw) (`GameplayStatics.GetWorldDeltaSeconds`) 10.0) false)))