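; BPC_EnemyStats is a health and stamina component that, despite its name, expects a BP_Player owner and drives that player's HUD.
; A tick after BeginPlay it caches the player and refreshes the HUD if the widget is valid.
; Decrease functions subtract and return true on depletion, while Increase functions cap at the maximum.
; Value changes push health and stamina ratios to the progress bars via UpdateHUDState.
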(event `self.ReceiveBeginPlay`
  (`KismetSystemLibrary.DelayUntilNextTick`)
  (bind _asbp_player (cast `/Game/Blueprints/HD/BP_Player` (`self.GetOwner`)))
  (bind _output_get (set `self.Player BP` _asbp_player))
  (`/Game/Blueprints/HD/BP_Player.HUD Widget` _output_get
    (:`then`
      (`self.Update HUD State`))
    (:`else`)))

(fn `Decrease Current Health`
  (params (Damage :type "Float (double-precision)"))
  (returns (`Is Player Dead` :type Boolean))
  (if (not (<= (`self.Current Health`) 0.0))
    (set `self.Current Health` (- (`self.Current Health`) Damage))
    (`self.Update HUD State`)
    (if (<= (`self.Current Health`) 0.0)
      _
      (else
        (return false)))
    (else
      (set `self.Current Health` 0.0)))
  (return true))

(fn `Decrease Current Stamina`
  (params (`Stamina Cost` :type "Float (double-precision)"))
  (returns (`Is Stamina Zero` :type Boolean))
  (if (not (<= (`self.Current Stamina`) 0.0))
    (set `self.Current Stamina` (- (`self.Current Stamina`) `Stamina Cost`))
    (`self.Update HUD State`)
    (if (<= (`self.Current Stamina`) 0.0)
      _
      (else
        (return false)))
    (else
      (set `self.Current Stamina` 0.0)))
  (return true))

(fn `Increase Current Health`
  (params (`Added Health` :type "Float (double-precision)"))
  (set `self.Current Health` (+ (`self.Current Health`) `Added Health`))
  (if (not (<= (`self.Current Health`) (`self.Max Health`)))
    (set `self.Current Health` (`self.Max Health`)))
  (`self.Update HUD State`))

(fn `Increase Current Stamina`
  (params (`Added Stamina` :type "Float (double-precision)"))
  (set `self.Current Stamina` (+ (`self.Current Stamina`) `Added Stamina`))
  (if (not (<= (`self.Current Stamina`) (`self.Max Stamina`)))
    (set `self.Current Stamina` (`self.Max Stamina`)))
  (`self.Update HUD State`))

(fn `Update HUD State`
  (`ProgressBar.SetPercent` (`/Game/ArtSources/UI/WB_HUD.HealthBar` (`/Game/Blueprints/HD/BP_Player.HUD Widget` (`self.Player BP`))) (/ (`self.Current Health`) (`self.Max Health`)))
  (`ProgressBar.SetPercent` (`/Game/ArtSources/UI/WB_HUD.StaminaBar` (`/Game/Blueprints/HD/BP_Player.HUD Widget` (`self.Player BP`))) (/ (`self.Current Stamina`) (`self.Max Stamina`))))