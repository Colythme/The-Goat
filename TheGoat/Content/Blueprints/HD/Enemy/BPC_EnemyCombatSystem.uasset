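; Combat component for BP_BOSS that runs its phase 1 attacks and hit reactions, turning it toward the player while idle.
; Combo and attack indices select montages, with CurrentAttackName (currently always Phase1Combo0101) keying the damage data table.
; Sword sphere traces damage the player, with a bonus at full rage.
; Incoming hits update health and rage, and higher impacts interrupt combos with staggers or knockdown.
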(event `Start Attack Combo`
  (params (`Combo Index` :type Integer))
  (if (`self.Can Attack?`)
    (set `self.Is Attacking?` true)
    (set `self.Current Combo Index` `Combo Index`)
    (`self.Rotate to Player` 10.0)
    (set `self.Attack Index` 0)
    (`self.Combo Selection`)))

(event `Attack Combo Next`
  (if (`self.Can Attack?`)
    (set `self.Attack Index` (+ (`self.Attack Index`) 1))
    (`self.Combo Selection`)))

(event `Stop Combo`
  (set `self.Is Attacking?` false)
  (set `self.Attack Index` 0)
  (`/Game/Blueprints/HD/Enemy/BP_BOSS.Set Whole Body Overlay Material` (`self.Boss BP`) "/Game/ArtSources/Materials/M_ActorGlow.M_ActorGlow")
  (`BlackboardComponent.SetValueAsBool` (`AIBlueprintHelperLibrary.GetBlackboard` (`self.Boss BP`)) "Is Attacking?" false))

(event `Phase 1 Combo 01 01`
  (params (StartingPosition :type "Float (single-precision)"))
  (`/Engine/EditorBlueprintResources/StandardMacros.DoOnce` false :!label _label
    (:`Completed`
      (`KismetSystemLibrary.Delay` 0.1)
      (`|PlayMontage` (`self.Boss Mesh`) "/Game/Animations/BOSS/Raw_UE4/Attack/Phase1/Combo_01/Combo_01_01_Montage.Combo_01_01_Montage" 0.7 StartingPosition
        (:`then`
          (goto _label :!via `Reset`))))))

(event `Phase 1 Combo 01 02`
  (params (StartingPosition :type "Float (single-precision)"))
  (`/Engine/EditorBlueprintResources/StandardMacros.DoOnce` false :!label _label_2
    (:`Completed`
      (`KismetSystemLibrary.Delay` 0.1)
      (`|PlayMontage` (`self.Boss Mesh`) "/Game/Animations/BOSS/Raw_UE4/Attack/Phase1/Combo_01/Combo_01_02_Montage.Combo_01_02_Montage" 0.5 StartingPosition
        (:`then`
          (goto _label_2 :!via `Reset`))))))

(event `Phase 1 Combo 01 03`
  (params (StartingPosition :type "Float (single-precision)"))
  (`/Engine/EditorBlueprintResources/StandardMacros.DoOnce` false :!label _label_3
    (:`Completed`
      (`KismetSystemLibrary.Delay` 0.1)
      (`|PlayMontage` (`self.Boss Mesh`) "/Game/Animations/BOSS/Raw_UE4/Attack/Phase1/Combo_01/Combo_01_03_Montage.Combo_01_03_Montage" 0.7 StartingPosition
        (:`then`
          (goto _label_3 :!via `Reset`))))))

(event `Phase 1 Combo 01 04`
  (params (StartingPosition :type "Float (single-precision)"))
  (`/Engine/EditorBlueprintResources/StandardMacros.DoOnce` false :!label _label_4
    (:`Completed`
      (`KismetSystemLibrary.Delay` 0.1)
      (`|PlayMontage` (`self.Boss Mesh`) "/Game/Animations/BOSS/Raw_UE4/Attack/Phase1/Combo_01/Combo_01_04_Montage.Combo_01_04_Montage" 0.8 StartingPosition
        (:`then`
          (goto _label_4 :!via `Reset`))))))

(event `Phase 1 Combo 01 05`
  (params (StartingPosition :type "Float (single-precision)"))
  (`/Engine/EditorBlueprintResources/StandardMacros.DoOnce` false :!label _label_5
    (:`Completed`
      (`KismetSystemLibrary.Delay` 0.1)
      (`|PlayMontage` (`self.Boss Mesh`) "/Game/Animations/BOSS/Raw_UE4/Attack/Phase1/Combo_01/Combo_01_05_Montage.Combo_01_05_Montage" 0.8 StartingPosition
        (:`then`
          (goto _label_5 :!via `Reset`))))))

(event `Phase 1 Combo 02 01`
  (params (StartingPosition :type "Float (single-precision)"))
  (`/Engine/EditorBlueprintResources/StandardMacros.DoOnce` false :!label _label_6
    (:`Completed`
      (`KismetSystemLibrary.Delay` 0.1)
      (`|PlayMontage` (`self.Boss Mesh`) "/Game/Animations/BOSS/Raw_UE4/Attack/Phase1/Combo_02/Combo_02_01_Montage.Combo_02_01_Montage" 1.0 StartingPosition
        (:`then`
          (goto _label_6 :!via `Reset`))))))

(event `Dodge Back`
  (`/Engine/EditorBlueprintResources/StandardMacros.DoOnce` false :!label _label_7
    (:`Completed`
      (`KismetSystemLibrary.Delay` 0.1)
      (`|PlayMontage` (`self.Boss Mesh`) "/Game/Animations/BOSS/Raw_UE4/Dodge/Dodge_Back_Montage.Dodge_Back_Montage"
        (:`then`
          (goto _label_7 :!via `Reset`))))))

(event `Phase 1 Combo 02 02`
  (params (StartingPosition :type "Float (single-precision)"))
  (`/Engine/EditorBlueprintResources/StandardMacros.DoOnce` false :!label _label_8
    (:`Completed`
      (`KismetSystemLibrary.Delay` 0.1)
      (`|PlayMontage` (`self.Boss Mesh`) "/Game/Animations/BOSS/Raw_UE4/Attack/Phase1/Combo_02/Combo_02_02_Montage.Combo_02_02_Montage" 0.8 StartingPosition
        (:`then`
          (goto _label_8 :!via `Reset`))))))

(event `Phase 1 Combo 02 03`
  (params (StartingPosition :type "Float (single-precision)"))
  (`/Engine/EditorBlueprintResources/StandardMacros.DoOnce` false :!label _label_9
    (:`Completed`
      (`KismetSystemLibrary.Delay` 0.1)
      (`|PlayMontage` (`self.Boss Mesh`) "/Game/Animations/BOSS/Raw_UE4/Attack/Phase1/Combo_02/Combo_02_03_Montage.Combo_02_03_Montage" 0.8 StartingPosition
        (:`then`
          (goto _label_9 :!via `Reset`))))))

(event `Phase 1 Combo 02 04`
  (params (StartingPosition :type "Float (single-precision)"))
  (`/Engine/EditorBlueprintResources/StandardMacros.DoOnce` false :!label _label_10
    (:`Completed`
      (`KismetSystemLibrary.Delay` 0.1)
      (`|PlayMontage` (`self.Boss Mesh`) "/Game/Animations/BOSS/Raw_UE4/Attack/Phase1/Combo_02/Combo_02_04_Montage.Combo_02_04_Montage" 0.8 StartingPosition
        (:`then`
          (goto _label_10 :!via `Reset`))))))

(event `Phase 1 Combo 02 05`
  (params (StartingPosition :type "Float (single-precision)"))
  (`/Engine/EditorBlueprintResources/StandardMacros.DoOnce` false :!label _label_11
    (:`Completed`
      (`KismetSystemLibrary.Delay` 0.1)
      (`|PlayMontage` (`self.Boss Mesh`) "/Game/Animations/BOSS/Raw_UE4/Attack/Phase1/Combo_02/Combo_02_05_Montage.Combo_02_05_Montage" 0.8 StartingPosition
        (:`then`
          (goto _label_11 :!via `Reset`))))))

(event `Phase 1 Chase Attack Ground Anim`
  (params (StartingPosition :type "Float (single-precision)"))
  (`/Engine/EditorBlueprintResources/StandardMacros.DoOnce` false :!label _label_12
    (:`Completed`
      (`KismetSystemLibrary.Delay` 0.1)
      (`|PlayMontage` (`self.Boss Mesh`) "/Game/Animations/BOSS/Raw_UE4/Attack/Phase1/ChaseAttack/ChaseAttack_Ground_Montage.ChaseAttack_Ground_Montage" 0.7 StartingPosition
        (:`then`
          (goto _label_12 :!via `Reset`))))))

(event `Phase 1 Chase Attack Air Anim`
  (params (StartingPosition :type "Float (single-precision)"))
  (`/Engine/EditorBlueprintResources/StandardMacros.DoOnce` false :!label _label_13
    (:`Completed`
      (`KismetSystemLibrary.Delay` 0.1)
      (`|PlayMontage` (`self.Boss Mesh`) "/Game/Animations/BOSS/Raw_UE4/Attack/Phase1/ChaseAttack/ChaseAttack_Air_Montage.ChaseAttack_Air_Montage" 0.7 StartingPosition
        (:`then`
          (goto _label_13 :!via `Reset`))))))

(event `Phase 1 Combo 03 02`
  (params (StartingPosition :type "Float (single-precision)"))
  (`/Engine/EditorBlueprintResources/StandardMacros.DoOnce` false :!label _label_14
    (:`Completed`
      (`KismetSystemLibrary.Delay` 0.1)
      (`|PlayMontage` (`self.Boss Mesh`) "/Game/Animations/BOSS/Raw_UE4/Attack/Phase1/Combo_03/Phase_1_Combo_03_02_Montage.Phase_1_Combo_03_02_Montage" 0.7 StartingPosition
        (:`then`
          (goto _label_14 :!via `Reset`))))))

(event `Phase 1 Combo 04 01`
  (params (StartingPosition :type "Float (single-precision)"))
  (`/Engine/EditorBlueprintResources/StandardMacros.DoOnce` false :!label _label_15
    (:`Completed`
      (`KismetSystemLibrary.Delay` 0.1)
      (`|PlayMontage` (`self.Boss Mesh`) "/Game/Animations/BOSS/Raw_UE4/Attack/Phase1/Combo_04/Phase_1_Combo_04_01_Montage.Phase_1_Combo_04_01_Montage" 0.6 StartingPosition
        (:`then`
          (goto _label_15 :!via `Reset`))))))

(event `Phase 1 Combo 05 01`
  (params (StartingPosition :type "Float (single-precision)"))
  (`/Engine/EditorBlueprintResources/StandardMacros.DoOnce` false :!label _label_16
    (:`Completed`
      (`KismetSystemLibrary.Delay` 0.1)
      (`|PlayMontage` (`self.Boss Mesh`) "/Game/Animations/BOSS/Raw_UE4/Attack/Phase1/Combo_05/Phase_1_Combo_05_01_Montage.Phase_1_Combo_05_01_Montage" 0.8 StartingPosition
        (:`then`
          (goto _label_16 :!via `Reset`))))))

(event `Phase 1 Combo 06 01`
  (params (StartingPosition :type "Float (single-precision)"))
  (`/Engine/EditorBlueprintResources/StandardMacros.DoOnce` false :!label _label_17
    (:`Completed`
      (`KismetSystemLibrary.Delay` 0.1)
      (`|PlayMontage` (`self.Boss Mesh`) "/Game/Animations/BOSS/Raw_UE4/Attack/Phase1/Combo_06/Phase_1_Combo_06_01_Montage.Phase_1_Combo_06_01_Montage" 1.0 StartingPosition
        (:`then`
          (goto _label_17 :!via `Reset`))))))

(event `Phase 1 Combo 01`
  (switch `int` (`self.Attack Index`)
    (:`0`
      (`self.Phase 1 Combo 01 01` 0.0)
      (set `self.Current Attack Name` "Phase1Combo0101"))
    (:`1`
      (`self.Phase 1 Combo 01 02` 0.2)
      (set `self.Current Attack Name` "Phase1Combo0101"))
    (:`2`
      (`self.Phase 1 Combo 01 03` 0.2)
      (set `self.Current Attack Name` "Phase1Combo0101"))
    (:`3`
      (`self.Phase 1 Combo 01 04` 0.2)
      (set `self.Current Attack Name` "Phase1Combo0101"))
    (:`4`
      (`self.Phase 1 Combo 01 05` 0.2)
      (set `self.Current Attack Name` "Phase1Combo0101"))))

(event `Phase 1 Combo 02`
  (switch `int` (`self.Attack Index`)
    (:`0`
      (`self.Phase 1 Combo 02 02` 0.0)
      (set `self.Current Attack Name` "Phase1Combo0101"))
    (:`1`
      (`self.Phase 1 Combo 02 03` 0.3)
      (set `self.Current Attack Name` "Phase1Combo0101"))
    (:`2`
      (`self.Phase 1 Combo 02 04` 0.3)
      (set `self.Current Attack Name` "Phase1Combo0101"))
    (:`3`
      (`self.Phase 1 Combo 02 05` 0.2)
      (set `self.Current Attack Name` "Phase1Combo0101"))))

(event `Phase 1 Chase Attack Ground`
  (switch `int` (`self.Attack Index`)
    (:`0`
      (`self.Phase 1 Chase Attack Ground Anim` 0.0)
      (set `self.Current Attack Name` "Phase1Combo0101"))))

(event `Phase 1 Chase Attack Air`
  (switch `int` (`self.Attack Index`)
    (:`0`
      (`self.Phase 1 Chase Attack Air Anim` 0.0)
      (set `self.Current Attack Name` "Phase1Combo0101"))))

(event `Phase 1 Combo 03`
  (switch `int` (`self.Attack Index`)
    (:`0`
      (`self.Phase 1 Combo 03 02` 0.0)
      (set `self.Current Attack Name` "Phase1Combo0101"))))

(event `Phase 1 Combo 04`
  (switch `int` (`self.Attack Index`)
    (:`0`
      (`self.Phase 1 Combo 04 01` 0.0)
      (set `self.Current Attack Name` "Phase1Combo0101"))))

(event `Phase 1 Combo 05`
  (switch `int` (`self.Attack Index`)
    (:`0`
      (`self.Phase 1 Combo 05 01` 0.0)
      (set `self.Current Attack Name` "Phase1Combo0101"))))

(event `Phase 1 Combo 06`
  (switch `int` (`self.Attack Index`)
    (:`0`
      (`self.Phase 1 Combo 06 01` 0.0)
      (set `self.Current Attack Name` "Phase1Combo0101"))))

(event `Combo Selection`
  (switch `int` (`self.Current Combo Index`)
    (:`1`
      (`self.Phase 1 Combo 01`))
    (:`2`
      (`self.Phase 1 Combo 02`))
    (:`3`
      (`self.Phase 1 Chase Attack Ground`))
    (:`4`
      (`self.Phase 1 Chase Attack Air`))
    (:`5`
      (`self.Phase 1 Combo 03`))
    (:`6`
      (`self.Dodge Back`))
    (:`7`
      (`self.Phase 1 Combo 04`))
    (:`8`
      (`self.Phase 1 Combo 05`))
    (:`9`
      (`self.Phase 1 Combo 06`))))

(event `Start Sword Trace`
  (bind _returnvalue (`KismetSystemLibrary.K2_SetTimerDelegate` :`Time` 0.005 :`bLooping` true))
  (set `self.Sword Trace Loop Timer` _returnvalue))

(event `Sword Trace Loop 1`
  (params (`Is RIght Hand Sword?` :type Boolean))
  (bind _boss_bp (`self.Boss BP`))
  (if `Is RIght Hand Sword?`
    (set `self.Current Sword Top Point` (`SceneComponent.K2_GetComponentLocation` (`/Game/Blueprints/HD/Enemy/BP_BOSS.Right Sword Top Point` (`self.Boss BP`))))
    (set `self.Current Sword Bottom Point` (`SceneComponent.K2_GetComponentLocation` (`/Game/Blueprints/HD/Enemy/BP_BOSS.Right Sword Bottom Point` (`self.Boss BP`))))
    (else
      (set `self.Current Sword Top Point` (`SceneComponent.K2_GetComponentLocation` (`/Game/Blueprints/HD/Enemy/BP_BOSS.Left Sword Top Point` (`self.Boss BP`))))
      (set `self.Current Sword Bottom Point` (`SceneComponent.K2_GetComponentLocation` (`/Game/Blueprints/HD/Enemy/BP_BOSS.Left Sword Bottom Point` (`self.Boss BP`))))))
  (bind (_outhit _returnvalue) (`KismetSystemLibrary.SphereTraceSingle` :`Start` (`self.Current Sword Bottom Point`) :`End` (`self.Current Sword Top Point`) :`Radius` 100.0 :`TraceChannel` "TraceTypeQuery1" :`DrawTime` 0.5))
  (if _returnvalue
    (bind (_bblockinghit _binitialoverlap _time _distance _location _impactpoint _normal _impactnormal _physmat _hitactor) (`GameplayStatics.BreakHitResult` _outhit))
    (if (`Actor.ActorHasTag` _hitactor "Player")
      (`/Engine/EditorBlueprintResources/StandardMacros.DoOnce` false :!label _label_18
        (:`Completed`
          (bind _angle (`self.Calc Angle Between Vectors` (`Actor.GetActorForwardVector` (`self.Boss BP`)) (`Actor.GetActorForwardVector` (`/Game/Blueprints/HD/Enemy/BP_BOSS.Player BP` (`self.Boss BP`)))))
          (bind _returnvalue_2 (`|GetDataTableRow` "/Game/Data/Data/BossAttack.BossAttack" (`self.Current Attack Name`))
            (:`then`
              (bind (_damage _tenacitydamage _defendrageincrease _impact _defendstaminacost) (break `/Game/Data/S_EnemyAttack` _returnvalue_2))
              (`/Game/Blueprints/HD/BPC_CombatSystem.Player Got Hit` (`/Game/Blueprints/HD/BP_Player.BPC_CombatSystem` (`/Game/Blueprints/HD/Enemy/BP_BOSS.Player BP` _boss_bp)) _boss_bp (+ _damage (* _damage (* (`/Game/Blueprints/HD/Enemy/BPC_EnemyStats.Is Rage Full?` (`self.BPC Enemy Stats`)) 0.5))) _tenacitydamage _defendstaminacost _angle _impact _defendrageincrease _location)
              (`KismetSystemLibrary.Delay` 0.5)
              (goto _label_18 :!via `Reset`))))))))

(event `Stop Sword Trace`
  (`KismetSystemLibrary.K2_ClearAndInvalidateTimerHandle` (`self.Sword Trace Loop Timer`)))

(event `Hit Index 01 Combat`
  (`/Game/Blueprints/HD/Enemy/BP_BOSS.Hit Index 01` (`self.Boss BP`)))

(event `Hit Index 02 Combat`
  (`self.Stop Combo`)
  (`/Game/Blueprints/HD/Enemy/BP_BOSS.Set Blackboard Hit` (`self.Boss BP`) true)
  (`|PlayMontage` (`self.Boss Mesh`) "/Game/Animations/BOSS/Raw_UE4/Hit/Hit_Impact_2_Montage.Hit_Impact_2_Montage"))

(event `Hit Index 03 Combat`
  (`self.Stop Combo`)
  (`/Game/Blueprints/HD/Enemy/BP_BOSS.Set Blackboard Hit` (`self.Boss BP`) true)
  (bind _angle (`self.Calc Angle Between Vectors` (`Actor.GetActorForwardVector` (`self.Boss BP`)) (- (`Actor.K2_GetActorLocation` (`/Game/Blueprints/HD/Enemy/BP_BOSS.Player BP` (`self.Boss BP`))) (`Actor.K2_GetActorLocation` (`self.Boss BP`)))))
  (if (> _angle 90.0)
    (`|PlayMontage` (`self.Boss Mesh`) "/Game/Animations/BOSS/Raw_UE4/Hit/Hit_Impact_3_B_Montage.Hit_Impact_3_B_Montage")
    (else
      (`|PlayMontage` (`self.Boss Mesh`) "/Game/Animations/BOSS/Raw_UE4/Hit/Hit_Impact_3_F_Montage.Hit_Impact_3_F_Montage"))))

(event `Hit Index 04 Combat`
  (`Character.StopAnimMontage` (`self.Boss BP`) null)
  (`self.Stop Combo`)
  (`/Game/Blueprints/HD/Enemy/BP_BOSS.Set Blackboard Hit` (`self.Boss BP`) true)
  (`|PlayMontage` (`self.Boss Mesh`) "/Game/Animations/BOSS/Raw_UE4/Hit/Knock_Down_Instance_Montage.Knock_Down_Instance_Montage"
    (:`OnBlendOut`
      (`|PlayMontage` (`self.Boss Mesh`) "/Game/Animations/BOSS/Raw_UE4/Hit/Knock_Down_Montage.Knock_Down_Montage"
        (:`OnBlendOut`
          (`|PlayMontage` (`self.Boss Mesh`) "/Game/Animations/BOSS/Raw_UE4/Hit/Knock_Down_Loop_Montage.Knock_Down_Loop_Montage"
            (:`then`
              (`CapsuleComponent.SetCapsuleSize` (`Character.CapsuleComponent` (`self.Boss BP`)) 50.0 88.0 true)
              (`KismetSystemLibrary.Delay` 3.0)
              (`|PlayMontage` (`self.Boss Mesh`) "/Game/Animations/BOSS/Raw_UE4/Hit/Knock_Down_GetUp_Montage.Knock_Down_GetUp_Montage"
                (:`then`
                  (`CapsuleComponent.SetCapsuleSize` (`Character.CapsuleComponent` (`self.Boss BP`)) 34.0 88.0 true))))))))))

(event `Hit Index 05 Combat`
  (`self.Stop Combo`)
  (`/Game/Blueprints/HD/Enemy/BP_BOSS.Set Blackboard Hit` (`self.Boss BP`) true)
  (`|PlayMontage` (`self.Boss Mesh`) "/Game/Animations/BOSS/Raw_UE4/Hit/FoughtBack/Hit_FoughtBack_1_Montage.Hit_FoughtBack_1_Montage" 0.6
    (:`OnBlendOut`
      (`|PlayMontage` (`self.Boss Mesh`) "/Game/Animations/BOSS/Raw_UE4/Hit/FoughtBack/Hit_FoughtBack_2_Montage.Hit_FoughtBack_2_Montage" 0.6))))

(event `Hit Index 04_1 Combat`
  (`self.Stop Combo`)
  (`/Game/Blueprints/HD/Enemy/BP_BOSS.Set Blackboard Hit` (`self.Boss BP`) true)
  (`|PlayMontage` (`self.Boss Mesh`) "/Game/Animations/BOSS/Raw_UE4/Hit/Hit_Impact_4_1_Montage.Hit_Impact_4_1_Montage"))

(event `FIghtBack Dealer`
  (bind _returnvalue (`|GetDataTableRow` "/Game/Data/Data/PlayerAttack.PlayerAttack" "FightBack")
    (:`then`
      (`self.Enemy Got Hit` (`.Damage_12_7C20B16648CEFF61BC4BB1A22DA4625C` (break `/Game/Data/S_PlayerAttack` _returnvalue)) 0.0 0 (`Actor.K2_GetActorLocation` (`self.Boss BP`))))))

(event `self.ReceiveBeginPlay`
  (bind _asbp_boss (cast `/Game/Blueprints/HD/Enemy/BP_BOSS` (`self.GetOwner`)))
  (bind _output_get (set `self.Boss BP` _asbp_boss))
  (set `self.Boss Mesh` (`Character.Mesh` _output_get))
  (set `self.BPC Enemy Stats` (`/Game/Blueprints/HD/Enemy/BP_BOSS.BPC_EnemyStats` (`self.Boss BP`))))

(event `self.ReceiveTick`
  (params (DeltaSeconds :type "Float (single-precision)"))
  (`|ExecutionSequence`
    (:`then_0`
      (if (`self.Is Attacking?`)
        _
        (elif (not (`self.Is Knocked Down`))
          (`self.Rotate to Player` 10.0))))))

(fn `Calc Angle Between Vectors`
  (params (VecA :type "Vector Structure") (VecB :type "Vector Structure"))
  (returns (Angle :type "Float (double-precision)"))
  (return (`KismetMathLibrary.DegAcos` (`KismetMathLibrary.Dot_VectorVector` (`KismetMathLibrary.Normal` VecA) (`KismetMathLibrary.Normal` VecB)))))

(fn `Commit Attack`
  (params (`Combo Index` :type Integer))
  (if (not (`self.Is Attacking?`))
    (`self.Start Attack Combo` `Combo Index`)))

(fn `Enemy Got Hit`
  (params (Damage :type "Float (double-precision)") (`Rage Bar Increase` :type "Float (double-precision)") (Impact :type Integer) (`Hit Location` :type "Vector Structure"))
  (locals (`C Damage` :type "Float (double-precision)") (`C Rage Bar Increase` :type "Float (double-precision)") (`C Impact` :type Integer) (`C Hit Location` :type "Vector Structure"))
  (set `local.C Damage` Damage)
  (set `local.C Rage Bar Increase` `Rage Bar Increase`)
  (set `local.C Impact` Impact)
  (set `local.C Hit Location` `Hit Location`)
  (`|ExecutionSequence`
    (:`then_0`
      (`/Game/Blueprints/HD/Enemy/BPC_EnemyStats.Decrease Current Health` (`self.BPC Enemy Stats`) (`local.C Damage`))
      (`/Game/Blueprints/HD/Enemy/BPC_EnemyStats.Increase Current Rage` (`self.BPC Enemy Stats`) (`local.C Rage Bar Increase`))
      (`NiagaraFunctionLibrary.SpawnSystemAtLocation` "/Game/Blood_VFX_Pack/Particles/Systems/P_SplashWithBurst_03.P_SplashWithBurst_03" (`local.C Hit Location`) (struct :`Yaw` -90.0)))
    (:`then_1`
      (if (> (`local.C Impact`) 0)
        (`self.Hit Index 01 Combat`)
        (if (not (`self.Is Knocked Down`))
          (switch `int` (`local.C Impact`)
            (:`2`
              (set `self.Can Attack?` false)
              (`self.Hit Index 02 Combat`))
            (:`3`
              (set `self.Can Attack?` false)
              (`self.Hit Index 03 Combat`))
            (:`4`
              (set `self.Can Attack?` false)
              (`self.Hit Index 04 Combat`))))))
    (:`then_2`
      (`GameplayStatics.PlaySound2D` "/Game/Blueprints/HD/Sound/Player/Hit/MS_HitBlood.MS_HitBlood" 1.0 1.0 0.0 null null))))

(fn `Rotate to Player`
  (params (InterpSpeed :type "Float (single-precision)" :default 10.0))
  (bind _boss_bp (`self.Boss BP`))
  (bind (_returnvalue_roll _returnvalue_pitch _returnvalue_yaw) (`KismetMathLibrary.BreakRotator` (`KismetMathLibrary.FindLookAtRotation` (`Actor.K2_GetActorLocation` _boss_bp) (`Actor.K2_GetActorLocation` (`/Game/Blueprints/HD/Enemy/BP_BOSS.Player BP` (`self.Boss BP`))))))
  (`Actor.K2_SetActorRotation` _boss_bp (`KismetMathLibrary.RInterpTo` (`Actor.K2_GetActorRotation` (`self.Boss BP`)) (`KismetMathLibrary.MakeRotator` 0.0 0.0 _returnvalue_yaw) (`GameplayStatics.GetWorldDeltaSeconds`) InterpSpeed) false))